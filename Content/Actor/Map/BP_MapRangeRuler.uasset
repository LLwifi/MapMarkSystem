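; BP_MapRangeRuler is a placeable actor that measures a rectangular map area between two corner components and fits a map camera to it.
; The construction script positions the RightUp corner from DiagonalPoint in world or relative space, then derives map size and diagonal length.
; It sizes a spring arm and axis arrows to show the extent.
; A valid MapCameraActor gets attached, centered and widened to the longer side.
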(fn `UserConstructionScript`
  (bind _springarm (`self.SpringArm`))
  (bind _rightup (`self.RightUp`))
  (bind _diagonalpoint (`self.DiagonalPoint`))
  (bind (_x _y) (`KismetMathLibrary.BreakVector2D` (`self.MapSize`)))
  (bind _relativelocation (`SceneComponent.RelativeLocation` (`self.LeftDown`)))
  (bind _relativelocation_2 (`SceneComponent.RelativeLocation` (`self.RightUp`)))
  (bind _x_2 (.x (/ (`SceneComponent.RelativeLocation` (`self.RightUp`)) 5.0)))
  (bind _y_2 (.y (/ (`SceneComponent.RelativeLocation` (`self.RightUp`)) 5.0)))
  (`|ExecutionSequence`
    (:`then_0`
      ; 根据DiagonalPoint设置对角点的位置
      (if (`self.IsUseWroldPoint`)
        (`SceneComponent.K2_SetWorldLocation` _rightup _diagonalpoint false false)
        (else
          (`SceneComponent.K2_SetRelativeLocation` _rightup _diagonalpoint false false))))
    (:`then_1`
      ; 计算当前地图的信息（尺寸）
      (set `self.MapSize` (`KismetMathLibrary.MakeVector2D` (- (.x _relativelocation_2) (.x _relativelocation)) (- (.y _relativelocation_2) (.y _relativelocation))))
      (bind _output_get (set `self.DiagonalLength` (`KismetMathLibrary.VSize` (- _relativelocation _relativelocation_2))))
      (set `SpringArmComponent.TargetArmLength` _output_get _springarm)
      (`SceneComponent.K2_SetRelativeRotation` _springarm (`KismetMathLibrary.FindLookAtRotation` (`SceneComponent.RelativeLocation` (`self.RightUp`)) (`SceneComponent.RelativeLocation` (`self.LeftDown`))) false false)
      ; 修改摄像机Actor
      (bind _mapcameraactor (`self.MapCameraActor`)
        (:`then`
          (`self.K2_AttachToActor` _mapcameraactor self "None" "SnapToTarget" "SnapToTarget" "SnapToTarget" true)
          (`self.K2_SetActorRelativeLocation` _mapcameraactor (`KismetMathLibrary.MakeVector` (.x (/ (`SceneComponent.RelativeLocation` (`self.RightUp`)) 2.0)) (.y (/ (`SceneComponent.RelativeLocation` (`self.RightUp`)) 2.0))) false false)
          (`/MapMarkSystem/Actor/Map/BP_MapCameraActor.SetCameraWidth` _mapcameraactor (select `bool` (>= _x _y) :`false` _y :`true` _x :!type "Float (single-precision)")))
        (:`else`)))
    (:`then_2`
      (set `ArrowComponent.ArrowLength` _x_2 (`self.Arrow_X`))
      (set `ArrowComponent.ArrowLength` _x_2 (`self.Arrow_X1`))
      (set `ArrowComponent.ArrowLength` _y_2 (`self.Arrow_Y`))
      (set `ArrowComponent.ArrowLength` _y_2 (`self.Arrow_Y1`)))))
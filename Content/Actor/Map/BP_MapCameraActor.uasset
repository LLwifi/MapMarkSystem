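; BP_MapCameraActor is an orthographic scene capture camera, apparently for rendering the game map.
; Its Construction Script clears the capture component's hidden list, then scans all actors in the level and hides those tagged HideActorFromMapCameraActor from the capture.
; SetCameraWidth lets callers set the capture's ortho width, while the event graph holds only disabled default events.
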(fn `SetCameraWidth`
  (params (`Ortho Width` :type "Float (single-precision)"))
  (set `SceneCaptureComponent2D.OrthoWidth` `Ortho Width` (`self.SceneCaptureComponent2D`)))

(fn `UserConstructionScript`
  (`SceneCaptureComponent.ClearHiddenComponents` (`self.SceneCaptureComponent2D`))
  (bind _outactors (`GameplayStatics.GetAllActorsOfClass` "/Script/Engine.Actor"))
  (for _array_element _outactors
    (if (`KismetArrayLibrary.Array_Contains` (`Actor.Tags` _array_element) "HideActorFromMapCameraActor")
      (`KismetArrayLibrary.Array_Add` (`SceneCaptureComponent.HiddenActors` (`self.SceneCaptureComponent2D`)) _array_element))))